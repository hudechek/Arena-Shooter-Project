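; BP_HealthPickup is an animated health pickup that heals the player or an enemy on overlap.
; Tick plays a timeline that scales the cube, whose update drives a second timeline that adds pitch and roll rotation.
; Box overlap casts to BP_PlayerCharacter to call both PlayerHealth and character Heal functions, falling back to BP_BaseEnemy's AIHeal.
; The graph neither destroys nor disables the pickup after use.
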(event OnComponentBeginOverlap(Box)
  (params (OverlappedComponent :type Primitive%20Component%20Object%20Reference) (OtherActor :type Actor%20Object%20Reference) (OtherComp :type Primitive%20Component%20Object%20Reference) (OtherBodyIndex :type Integer) (bFromSweep :type Boolean) (SweepResult :type Hit%20Result%20Structure%20%28by%20ref%29))
  ;[1 1 1] Cast to player or Ai character to call heal functions and player UI Health Vinegtte
  (bind _asbp_player_character (Utilities|Casting|CastToBP_PlayerCharacter OtherActor)
    (:then
      (Default|Heal (Variables|/Game/Player/BP_PlayerCharacter.BP_PlayerCharacter_C|GetPlayer%20health _asbp_player_character))
      (Default|Heal _asbp_player_character))
    (:CastFailed
      (bind _asbp_base_enemy (Utilities|Casting|CastToBP_BaseEnemy OtherActor))
      (Default|AIHeal _asbp_base_enemy))))

(event EventTick
  (params (DeltaSeconds :type Float%20%28single-precision%29))
  ;[1 1 1] Applay rotation and scale changes to mesh every tick
  (bind _newtrack_0 (Timeline|Timeline Play)
    (:Update
      (Transformation|SetWorldScale3D (Variables|Default|GetCube) (Math|Conversions|ToVector(Float) _newtrack_0))
      (bind _newtrack_0_2 (Timeline|Timeline_0 Play)
        (:Update
          (Transformation|AddWorldRotation (Variables|Default|GetCube) (Math|Rotator|MakeRotator _newtrack_0_2 _newtrack_0_2 0.0) false false))))))

(fn ConstructionScript)