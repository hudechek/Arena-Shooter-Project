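; BP_InvencibilityPickup is a pickup that grants invincibility to the player character or an AI enemy that overlaps its box.
; A player overlap calls InvincibilityTimer on the character and Invincible on its PlayerHealth to display the invincibility overlay.
; Otherwise, a BP_BaseEnemy overlap calls AiInvincibility.
; Tick plays a timeline that pulses the cube's world scale for visual distinction, and the pickup does not destroy itself here.
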(event OnComponentBeginOverlap(Box)
  (params (OverlappedComponent :type Primitive%20Component%20Object%20Reference) (OtherActor :type Actor%20Object%20Reference) (OtherComp :type Primitive%20Component%20Object%20Reference) (OtherBodyIndex :type Integer) (bFromSweep :type Boolean) (SweepResult :type Hit%20Result%20Structure%20%28by%20ref%29))
  ;[1 1 1] on overlap calls invincibility event from Ai or Player Character and displayes Player inviciblity overlay
  (bind _asbp_player_character (Utilities|Casting|CastToBP_PlayerCharacter OtherActor)
    (:then
      (Default|InvincibilityTimer _asbp_player_character)
      (Default|Invincible (Variables|/Game/Player/BP_PlayerCharacter.BP_PlayerCharacter_C|GetPlayer%20health _asbp_player_character)))
    (:CastFailed
      (bind _asbp_base_enemy (Utilities|Casting|CastToBP_BaseEnemy OtherActor))
      (Default|AiInvincibility _asbp_base_enemy))))

(event EventTick
  (params (DeltaSeconds :type Float%20%28single-precision%29))
  ;[1 1 1] Increses and decreses scale of pick up in world for visual distinction
  (bind _newtrack_0 (Timeline|Timeline Play)
    (:Update
      (Transformation|SetWorldScale3D (Variables|Default|GetCube) (Math|Conversions|ToVector(Float) _newtrack_0)))))

(fn ConstructionScript)