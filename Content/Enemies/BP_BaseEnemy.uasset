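; Base AI enemy for a scored shooter: it senses targets, fires projectiles on a looping timer, heals and picks a random name.
; AI perception writes the sensed actor to the Blackboard's Enemy Actor key.
; Damage updates a floating health bar that yaws toward the player.
; On death it credits the killing enemy or player, hides below the map, then moves to a random BP_SpawnPoint after a delay.
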(event OnTargetPerceptionUpdated(AIPerception)
  (params (Actor :type Actor%20Object%20Reference) (Stimulus :type AI%20Stimulus%20Structure))
  (bind _returnvalue (AI|GetBlackboard 0))
  (bind _returnvalue_2 (Utilities|Name|MakeLiteralName "Enemy Actor"))
  ;[1 1 1] Ai Preception
  (if (.bSuccessfullySensed (Utilities|Struct|BreakAIStimulus Stimulus))
    (bind _output_get (Variables|Default|SetTraget%20Enemy Actor))
    (Utilities|IsValid _returnvalue
      (:Is%20Valid
        (AI|Components|Blackboard|SetValueasObject _returnvalue _returnvalue_2 _output_get)))
    (else
      (Variables|Default|SetTraget%20Enemy 0)
      (AI|Components|Blackboard|SetValueasObject _returnvalue _returnvalue_2 0))))

(event Custom|Shoot
  ;[1 1 1] Spawns projectile
  (Game|SpawnActorfromClass "/Game/Enemies/Default_Enemy-Projectile.Default_Enemy-Projectile_C" (Transformation|GetWorldTransform (Variables|Default|GetProjectile%20direction)) "Undefined" "MultiplyWithRoot" self 0))

(event Custom|StartShoooting
  ;[1 1 1] Starts projectile spawning
  (Utilities|Time|SetTimerbyFunctionName 0 "Shoot" (Variables|Default|GetFireRate) true))

(event Custom|AiInvincibility
  ;[1 1 1] Invincibility timer
  (Variables|Default|SetIs%20Invincible true)
  (Utilities|FlowControl|Delay 5.0)
  (Variables|Default|SetIs%20Invincible false))

(event Custom|StopShotting
  ;[1 1 1] Stops projectiles
  (Utilities|Time|ClearTimerbyFunctionName 0 "Shoot"))

(event Custom|CheckHealth
  (bind _damage_causer (Variables|Default|GetDamage%20Causer))
  ;[1 1 1] AI Health system
  (if (<= (Variables|Default|GetCurrentHealth) 0.0)
    (bind _asbp_base_enemy (Utilities|Casting|CastToBP_BaseEnemy _damage_causer)
      (:then
        (CallFunction|AddtoAIScore _asbp_base_enemy 1))
      (:CastFailed
        (bind _asbp_player_character (Utilities|Casting|CastToBP_PlayerCharacter _damage_causer))
        (Default|AddtoScore _asbp_player_character 1)))
    (Transformation|SetActorLocation "0.000000,0.000000,-5000.000000" false false)
    (Variables|Default|SetCurrentHealth (Variables|Default|GetStartingHealth))
    (CallFunction|Respawn)))

(event Custom|Respawn
  (bind _out_actors (Variables|Default|GetOut%20Actors))
  ;[1 1 1] AI respawn
  (Utilities|FlowControl|Delay 5.0)
  (Variables|Default|SetCurrentHealth (Variables|Default|GetStartingHealth))
  (Transformation|SetActorLocation (Transformation|GetActorLocation (Utilities|Array|Get(acopy) _out_actors (Math|Random|RandomIntegerinRange 0 (- (Utilities|Array|Length _out_actors) 1)))) false false))

(event Custom|AddToAIScore
  (params (ValueToAdd :type Integer))
  ;[1 1 1] Add to score of AiCharcter
  (Variables|Default|SetScore (+ (Variables|Default|GetScore) ValueToAdd)))

(event Custom|AsignName
  (bind _ainames (Variables|Default|GetAiNames))
  ;[1 1 1] Absolutly redementary name array to from (same name is likely)
  (Variables|Default|SetName (Utilities|Array|Get(acopy) _ainames (Math|Random|RandomInteger (Utilities|Array|Length _ainames)))))

(event Custom|AIHeal
  ;[1 1 1] allows Ai to heal if pick up is  walked over
  (CallFunction|AIHealthReplenish)
  ;[1 1 1] AI Health system
  (Default|AIHealthBar (Variables|Default|GetAI_Healthbar) (Variables|Default|GetCurrentHealth) (Variables|Default|GetStartingHealth)))

(event Game|Damage|EventAnyDamage
  (params (Damage :type Float%20%28single-precision%29) (DamageType :type Damage%20Type%20Object%20Reference) (InstigatedBy :type Controller%20Object%20Reference) (DamageCauser :type Actor%20Object%20Reference))
  ;[1 1 1] AI Health system
  (Variables|Default|SetDamage%20Causer DamageCauser)
  (Variables|Default|SetCurrentHealth (- (Variables|Default|GetCurrentHealth) Damage))
  (CallFunction|CheckHealth)
  (Default|AIHealthBar (Variables|Default|GetAI_Healthbar) (Variables|Default|GetCurrentHealth) (Variables|Default|GetStartingHealth)))

(event EventBeginPlay
  ;[1 1 1] at the begain of gameplay call all spawn point actors and set them as an array of out actors, then cast to Ai_health widget and set AI Healthbar for floating health indicator, final call assign name function
  (bind _outactors (Actor|GetAllActorsOfClass "/Game/Spawner/BP_SpawnPoint.BP_SpawnPoint_C"))
  (Variables|Default|SetOut%20Actors _outactors)
  (bind _asai_health_bar (Utilities|Casting|CastToAI_HEalthBar (UserInterface|GetUserWidgetObject (Variables|Default|GetWidget))))
  (Variables|Default|SetAI_Healthbar _asai_health_bar)
  (CallFunction|AsignName))

(event EventTick
  (params (DeltaSeconds :type Float%20%28single-precision%29))
  (bind _widget (Variables|Default|GetWidget))
  ;[1 1 1] Makes Health of Ai visible to Player
  (Transformation|SetWorldRotation _widget (Math|Rotator|MakeRotator 0.0 0.0 (.yaw (Math|Rotator|FindLookatRotation (Transformation|GetWorldLocation _widget) (Transformation|GetActorLocation (Game|GetPlayerCharacter 0))))) false false))

(fn ConstructionScript)

(fn AIHealthReplenish
  (Variables|Default|SetCurrentHealth (Variables|Default|GetStartingHealth)))